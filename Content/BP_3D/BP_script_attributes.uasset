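; Test Blueprint that inspects Cesium feature metadata by clicking objects in the 3D scene.
; BeginPlay enables input, the mouse cursor, and click and hover events on the player controller.
; A left click reads property table values from a complex Visibility trace under the cursor and prints each key-value pair on screen.
; Unconnected line-trace and feature-ID lookup nodes remain as unused experiments.
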(event `Key|LeftMouseButton`
  (params (Key :type "Key Structure"))
  (bind _returnvalue (`CesiumMetadataValueBlueprintLibrary.GetValuesAsStrings` (`CesiumMetadataPickingBlueprintLibrary.GetPropertyTableValuesFromHit` (`PlayerController.GetHitResultUnderCursorByChannel` (`GameplayStatics.GetPlayerController` 0) "TraceTypeQuery1" true))))
  ; current test
  (:`Pressed`
    (bind _keys (`BlueprintMapLibrary.Map_Keys` _returnvalue))
    (for _array_element _keys
      (`KismetSystemLibrary.PrintString` (`KismetStringLibrary.Concat_StrStr` _array_element ":" (`BlueprintMapLibrary.Map_Find` _returnvalue _array_element)) true true (struct :`G` 0.66 :`B` 1.0 :`A` 1.0) 25.0))))

(event `self.ReceiveBeginPlay`
  (bind _returnvalue (`GameplayStatics.GetPlayerController` 0))
  ; Player controller
  (`self.EnableInput` _returnvalue)
  (set `PlayerController.bShowMouseCursor` true _returnvalue)
  (set `PlayerController.bEnableClickEvents` true _returnvalue)
  (set `PlayerController.bEnableMouseOverEvents` true _returnvalue))

(fn `UserConstructionScript`)