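; Click-to-inspect Blueprint for 3D buildings that reads feature metadata and queries a building energy REST API.
; BeginPlay enables cursor and click input on player controller 1, while left press line-traces from controller 0's mouse to print the hit's property table.
; Release stores the gml:id and prints the API URL.
; Press also sends a VaRest GET using the stored id, but its callback is empty and the energy-demand parsing is unwired.
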(event `self.ReceiveBeginPlay`
  (bind _returnvalue (`GameplayStatics.GetPlayerController` 1))
  ; Control the camera when executing actions
  (`self.EnableInput` _returnvalue)
  (set `PlayerController.bShowMouseCursor` true _returnvalue)
  (set `PlayerController.bEnableClickEvents` true _returnvalue)
  (set `PlayerController.bEnableMouseOverEvents` true _returnvalue))

(event `Key|LeftMouseButton`
  (params (Key :type "Key Structure"))
  (bind (_worldlocation _worlddirection) (`PlayerController.DeprojectMousePositionToWorld` (`GameplayStatics.GetPlayerController` 0)))
  ; Displaying attributes
  (:`Pressed`
    (bind _outhit (`KismetSystemLibrary.LineTraceSingle` :`Start` _worldlocation :`End` (+ (* _worlddirection 100000.0) _worldlocation) :`TraceChannel` "TraceTypeQuery1" :`DrawDebugType` "ForDuration"))
    (bind _returnvalue (`CesiumMetadataValueBlueprintLibrary.GetValuesAsStrings` (`CesiumMetadataPickingBlueprintLibrary.GetPropertyTableValuesFromHit` _outhit)))
    (bind _keys (`BlueprintMapLibrary.Map_Keys` _returnvalue))
    (for _array_element _keys
      (`KismetSystemLibrary.PrintString` (`KismetStringLibrary.Concat_StrStr` _array_element ":" (`BlueprintMapLibrary.Map_Find` _returnvalue _array_element)) true true (struct :`A` 1.0) 20.0)))
  (:`Released`
    ; Get the modified gml_id of the cliked building and construct the API URL for Building Energy information
    (bind _output_get (set `self.modified_gml_id` (`BlueprintMapLibrary.Map_Find` _returnvalue "gml:id")))
    (`KismetSystemLibrary.PrintString` (`KismetStringLibrary.Concat_StrStr` (`self.base_url_energy`) (`self.community_id`) "&" "modified_gml_id=" _output_get "&" "format=json") true true (struct :`G` 0.66 :`B` 1.0 :`A` 1.0) 20.0)))

(event `CustomEvent`
  (bind _returnvalue (`GameplayStatics.GetPlayerController` 0))
  ; Mouse events
  (`self.EnableInput` _returnvalue)
  (set `PlayerController.bShowMouseCursor` true _returnvalue)
  (set `PlayerController.bEnableClickEvents` true _returnvalue)
  (set `PlayerController.bEnableMouseOverEvents` true _returnvalue))

(event `Key|LeftMouseButton`
  (params (Key :type "Key Structure"))
  (bind _returnvalue (subsystem `VaRestSubsystem`))
  ; Get Building energy information and color
  (:`Pressed`
    (bind _returnvalue_2 (`VaRestSubsystem.ConstructVaRestJsonObject` _returnvalue))
    (`VaRestSubsystem.CallURL` _returnvalue (`KismetStringLibrary.Concat_StrStr` (`self.base_url_energy`) (`self.community_id`) "&" "modified_gml_id=" (stale _output_get) "&" "format=json") "GET" "x_www_form_urlencoded_url" _returnvalue_2 (delegate `RestCallback`))))

(event `RestCallback`
  (params (Request :type "VaRestRequestJSON Object Reference"))
  ; Get Building energy information and color
)

(fn `UserConstructionScript`)