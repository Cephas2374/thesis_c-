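; Building energy Blueprint that queries a web service for data by community ID and modified GML ID.
; BeginPlay enables input, cursor, click and hover events on the first player controller, duplicated in a custom event.
; Any left mouse press sends a VaRest GET with the concatenated URL, and the callback prints the raw response.
; Parsing of energy_demand is left unconnected, and no coloring logic exists yet.
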(event `self.ReceiveBeginPlay`
  (bind _returnvalue (`GameplayStatics.GetPlayerController` 0))
  ; Control the camera when executing actions
  (`self.EnableInput` _returnvalue)
  (set `PlayerController.bShowMouseCursor` true _returnvalue)
  (set `PlayerController.bEnableClickEvents` true _returnvalue)
  (set `PlayerController.bEnableMouseOverEvents` true _returnvalue))

(event `CustomEvent`
  (bind _returnvalue (`GameplayStatics.GetPlayerController` 0))
  ; Mouse events
  (`self.EnableInput` _returnvalue)
  (set `PlayerController.bShowMouseCursor` true _returnvalue)
  (set `PlayerController.bEnableClickEvents` true _returnvalue)
  (set `PlayerController.bEnableMouseOverEvents` true _returnvalue))

(event `Key|LeftMouseButton`
  (params (Key :type "Key Structure"))
  (bind _returnvalue (subsystem `VaRestSubsystem`))
  ; Reading the JSON
  (:`Pressed`
    (bind _returnvalue_2 (`VaRestSubsystem.ConstructVaRestJsonObject` _returnvalue))
    (`VaRestSubsystem.CallURL` _returnvalue (`KismetStringLibrary.Concat_StrStr` (`self.base_url`) "community_id=" (`self.community_id`) "&modified_gml_id=" (`self.modified_gml_id`)) "GET" "x_www_form_urlencoded_url" _returnvalue_2 (delegate `RestCallback`))))

(event `RestCallback`
  (params (Request :type "VaRestRequestJSON Object Reference"))
  ; Reading the JSON
  (bind _returnvalue (`VaRestRequestJSON.GetResponseContentAsString` Request true))
  (`KismetSystemLibrary.PrintString` _returnvalue))

(fn `UserConstructionScript`)