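; Actor script that logs into a backend and shows energy data for clicked buildings in a 3D tileset.
; BeginPlay POSTs credentials via VaRest, stores the returned access token on completion, and requests a building preload without awaiting it.
; Left press line-traces under the cursor and calls BuildingEnergyDisplay's fetch per feature-metadata key.
; Release stores the hit's gml:id afterwards, so each fetch uses the previously stored ID.
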(event `self.ReceiveBeginPlay`
  (bind _returnvalue (subsystem `VaRestSubsystem`))
  ; Authenticate Final
  (bind _returnvalue_2 (`VaRestSubsystem.ConstructVaRestJsonObject` _returnvalue))
  (`VaRestJsonObject.SetStringField` _returnvalue_2 "username" (`self.username`))
  (`VaRestJsonObject.SetStringField` _returnvalue_2 "password" (`self.password`))
  (bind _returnvalue_3 (`VaRestSubsystem.ConstructVaRestRequestExt` _returnvalue "POST" "json"))
  (`VaRestRequestJSON.SetHeader` _returnvalue_3 "Content-Type" "application/json")
  (`VaRestRequestJSON.SetHeader` _returnvalue_3 "Accept" "application/json")
  (`VaRestRequestJSON.SetRequestObject` _returnvalue_3 _returnvalue_2)
  (add `VaRestRequestJSON.OnRequestComplete` _returnvalue_3 (delegate `ReqCompleted`))
  (add `VaRestRequestJSON.OnRequestFail` _returnvalue_3 (delegate `AuthenticationFail`))
  (`VaRestRequestJSON.ProcessURL` _returnvalue_3 (`self.backend_login`))
  (`BuildingEnergyDisplay.PreloadAllBuildingData` (stale `Key|LeftMouseButton` _returnvalue_2) (stale `ReqCompleted` _output_get)))

(event `AuthenticationFail`
  (params (Request :type "VaRestRequestJSON Object Reference"))
  ; Authenticate Final
  (`KismetSystemLibrary.PrintString` (`|GetEnumeratorNameAsString` (`VaRestRequestJSON.GetStatus` Request)))
  (`KismetSystemLibrary.PrintString` (`KismetStringLibrary.Conv_IntToString` (`VaRestRequestJSON.GetResponseCode` Request))))

(event `ReqCompleted`
  (params (Request :type "VaRestRequestJSON Object Reference"))
  ; Authenticate Final
  (bind _output_get (set `self.access` (`VaRestJsonObject.GetStringField` (`VaRestRequestJSON.GetResponseObject` Request) "access")))
  (`KismetSystemLibrary.PrintString` _output_get true true (struct :`G` 0.66 :`B` 1.0 :`A` 1.0) 20.0))

(event `CustomEvent_0`
  (bind _returnvalue (`GameplayStatics.GetPlayerController` 0))
  ; Control the camera when executing actions
  (`self.EnableInput` _returnvalue)
  (set `PlayerController.bShowMouseCursor` true _returnvalue)
  (set `PlayerController.bEnableClickEvents` true _returnvalue)
  (set `PlayerController.bEnableMouseOverEvents` true _returnvalue))

(event `Key|LeftMouseButton`
  (params (Key :type "Key Structure"))
  (bind (_worldlocation _worlddirection) (`PlayerController.DeprojectMousePositionToWorld` (`GameplayStatics.GetPlayerController` 0)))
  ; Displaying attributes
  (:`Pressed`
    (bind _outhit (`KismetSystemLibrary.LineTraceSingle` :`Start` _worldlocation :`End` (+ (* _worlddirection 100000.0) _worldlocation) :`TraceChannel` "TraceTypeQuery1" :`DrawDebugType` "ForDuration"))
    (bind _returnvalue (`CesiumMetadataValueBlueprintLibrary.GetValuesAsStrings` (`CesiumMetadataPickingBlueprintLibrary.GetPropertyTableValuesFromHit` _outhit)))
    (bind _keys (`BlueprintMapLibrary.Map_Keys` _returnvalue))
    (for _array_element _keys
      (bind _returnvalue_2 (`GameplayStatics.GetActorOfClass` "/Script/Final_project.BuildingEnergyDisplay"))
      (`BuildingEnergyDisplay.FetchBuildingEnergyData` _returnvalue_2 (stale _output_get) (stale `ReqCompleted` _output_get))))
  (:`Released`
    ; Get the modified gml_id of the cliked building and construct the API URL for Building Energy information
    (bind _output_get (set `self.modified_gml_id` (`BlueprintMapLibrary.Map_Find` _returnvalue "gml:id")))
    (`KismetSystemLibrary.PrintString` _output_get)))

(event `CustomEvent`
  (bind _returnvalue (`GameplayStatics.GetPlayerController` 0))
  ; Mouse events
  (`self.EnableInput` _returnvalue)
  (set `PlayerController.bShowMouseCursor` true _returnvalue)
  (set `PlayerController.bEnableClickEvents` true _returnvalue)
  (set `PlayerController.bEnableMouseOverEvents` true _returnvalue))

(fn `UserConstructionScript`)