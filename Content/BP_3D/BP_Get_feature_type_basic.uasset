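; Test Blueprint that requests basic feature-type data for one hard-coded building from a GIS World geospatial buildings-energy backend.
; BeginPlay, and a duplicate custom event, enable input, the mouse cursor, click and mouse-over events.
; Left mouse press sends a VaRest GET to the fixed URL.
; The callback only extracts the first "id" array element as an object; response printing and geometry reading are unconnected.
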(event `self.ReceiveBeginPlay`
  (bind _returnvalue (`GameplayStatics.GetPlayerController` 0))
  ; Control the camera when executing actions
  (`self.EnableInput` _returnvalue)
  (set `PlayerController.bShowMouseCursor` true _returnvalue)
  (set `PlayerController.bEnableClickEvents` true _returnvalue)
  (set `PlayerController.bEnableMouseOverEvents` true _returnvalue))

(event `CustomEvent`
  (bind _returnvalue (`GameplayStatics.GetPlayerController` 0))
  ; Mouse events
  (`self.EnableInput` _returnvalue)
  (set `PlayerController.bShowMouseCursor` true _returnvalue)
  (set `PlayerController.bEnableClickEvents` true _returnvalue)
  (set `PlayerController.bEnableMouseOverEvents` true _returnvalue))

(event `Key|LeftMouseButton`
  (params (Key :type "Key Structure"))
  (bind _returnvalue (subsystem `VaRestSubsystem`))
  ; Reading the JSON
  (:`Pressed`
    (bind _returnvalue_2 (`VaRestSubsystem.ConstructVaRestJsonObject` _returnvalue))
    (`VaRestSubsystem.CallURL` _returnvalue "https://backend.gisworld-tech.com/geospatial/buildings-energy/DEBWL001000hyHDD/?community_id=08417008&field_type=basic&_ts=1764005996961" "GET" "x_www_form_urlencoded_body" _returnvalue_2 (delegate `RestCallback`))))

(event `RestCallback`
  (params (Request :type "VaRestRequestJSON Object Reference"))
  ; Reading the JSON
  (bind _returnvalue (`VaRestJsonValue.AsObject` (`|GetArrayItem` (`VaRestJsonObject.GetArrayField` (`VaRestRequestJSON.GetResponseObject` Request) "id")))))

(fn `UserConstructionScript`)